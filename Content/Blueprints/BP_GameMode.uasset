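; Game mode that spawns local players and handles the target-destruction goal leading to Level2.
; BeginPlay caches actors tagged TargetTag and calls CreatePlayer twice.
; UpdateDestroyedTargets loops over the targets, breaking at the first intact one, but the code after the loop still runs after a break, showing UI_WinLose and immediately opening Level2.
; ChoosePlayerStart is overridden but returns no start.
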(event `self.ReceiveBeginPlay`
  (bind _outactors (`GameplayStatics.GetAllActorsWithTag` "TargetTag"))
  (set `self.AllTargets` _outactors)
  (for _index (range 2)
    (`GameplayStatics.CreatePlayer` _index)))

(event `UpdateDestroyedTargets`
  ;[1 1 1] Check if all targets are destroyed, if they are, display win/lose screen
  (for _array_element (`self.AllTargets`)
    (bind _asbp_target (cast `/Game/Blueprints/Target/BP_Target` _array_element))
    (if (not (`/Game/Blueprints/Target/BP_Target.bIsDestroyed` _asbp_target))
      (break)))
  (`KismetSystemLibrary.PrintString` "All targets destroyed")
  (bind _returnvalue (`|CreateWidget` "/Game/Blueprints/UI/UI_WinLoSe.UI_WinLose_C"))
  (`UserWidget.AddToViewport` _returnvalue 0)
  (`GameplayStatics.OpenLevel` "Level2"))

(fn `ChoosePlayerStart`
  (params (Player :type "Controller Object Reference"))
  (returns (ReturnValue :type "Actor Object Reference"))
  (return null))

(fn `UserConstructionScript`)