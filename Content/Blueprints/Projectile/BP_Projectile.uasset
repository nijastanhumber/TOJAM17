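; BP_Projectile is a reusable projectile that bounces off mirrors and shield characters to destroy targets.
; Fire launches it along local X and, if it was hidden, shows it and clears InUse after a temporary delay.
; Tag-checked overlaps redirect it from the reflector's location along its forward vector, counting only mirror bounces.
; Target hits hide both actors and update BP_GameMode, while other hits stop and hide it unless Box has multiple overlaps.
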(event `self.ReceiveActorBeginOverlap`
  (params (OtherActor :type "Actor Object Reference"))
  ;[1 1 1] Hit Mirror
  (if (`self.ActorHasTag` OtherActor "PlayerTag")
    (if (`self.ActorHasTag` OtherActor "ShieldGuyTag")
      (bind _asbp_shield_character (cast `/Game/Blueprints/Characters/BP_ShieldCharacter` OtherActor))
      (`ProjectileMovementComponent.SetVelocityInLocalSpace` (`self.ProjectileMovement`) (* (`SceneComponent.GetForwardVector` (`/Game/Blueprints/Characters/BP_ShieldCharacter.ShieldMesh` _asbp_shield_character)) (`self.FireVelocityX`)))
      (`SceneComponent.K2_SetWorldLocation` (`self.DefaultSceneRoot`) (`self.K2_GetActorLocation` _asbp_shield_character) false false))
    (elif (`self.ActorHasTag` OtherActor "MirrorTag")
      (`self.K2_SetActorRotation` (struct))
      (bind _asbp_mirror (cast `/Game/Blueprints/Mirror/BP_Mirror` OtherActor))
      (`ProjectileMovementComponent.SetVelocityInLocalSpace` (`self.ProjectileMovement`) (* (`SceneComponent.GetForwardVector` (`/Game/Blueprints/Mirror/BP_Mirror.MirrorPlaceHolder` _asbp_mirror)) (`self.FireVelocityX`)))
      (`SceneComponent.K2_SetWorldLocation` (`self.DefaultSceneRoot`) (`self.K2_GetActorLocation` _asbp_mirror) false false)
      (bind _result (`/Engine/EditorBlueprintResources/StandardMacros.IncrementInt` (`self.numOfBounces`))
        (:`  `
          (set `self.numOfBounces` _result)))
      (else
        ;[1 1 1] Hit Target
        (if (`self.ActorHasTag` OtherActor "TargetTag")
          (`KismetSystemLibrary.PrintString` "HitTarget!")
          (set `self.bInUse` false)
          (`ProjectileMovementComponent.SetVelocityInLocalSpace` (`self.ProjectileMovement`) (0.0 0.0 0.0))
          (`self.SetActorHiddenInGame` true)
          (bind _asbp_target (cast `/Game/Blueprints/Target/BP_Target` OtherActor))
          (set `/Game/Blueprints/Target/BP_Target.bIsDestroyed` true _asbp_target)
          (`self.SetActorHiddenInGame` _asbp_target true)
          (bind _asbp_game_mode (cast `/Game/Blueprints/BP_GameMode` (`GameplayStatics.GetGameMode`)))
          (`/Game/Blueprints/BP_GameMode.UpdateDestroyedTargets` _asbp_game_mode)
          (else
            ;[1 1 1] Hit Everything else
            (if (not (> (`KismetArrayLibrary.Array_Length` (`PrimitiveComponent.GetOverlappingComponents` (`self.Box`))) 1))
              (`KismetSystemLibrary.PrintString` "hit wall")
              (set `self.bInUse` false)
              (`ProjectileMovementComponent.SetVelocityInLocalSpace` (`self.ProjectileMovement`) (0.0 0.0 0.0))
              (`self.SetActorHiddenInGame` true)
              (`self.K2_SetActorLocation` (0.0 0.0 0.0)))))))))

(event `Fire`
  ;[1 1 1] Fire
  (`ProjectileMovementComponent.SetVelocityInLocalSpace` (`self.ProjectileMovement`) (`KismetMathLibrary.MakeVector` (`self.FireVelocityX`)))
  (if (`self.bHidden`)
    (`self.SetActorHiddenInGame` false)
    ;[1 1 1] Temp
    (`KismetSystemLibrary.Delay` 1.0)
    (set `self.bInUse` false)))

(event `self.ReceiveBeginPlay`)

(fn `UserConstructionScript`)