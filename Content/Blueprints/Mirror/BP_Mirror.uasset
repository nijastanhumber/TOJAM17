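; BP_Mirror is an actor that tilts its root's pitch up or down in fixed steps within vertical limits.
; ChangeAngle updates the clamped TargetPitch, then a Gate and one-frame Delay loop moves pitch there at constant speed, stopping at the target or limit.
; Calls during movement only retarget the running loop.
; Actor overlap plays a one-shot bounce animation on the Tramp component.
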(event `self.ReceiveBeginPlay`
  (bind (_relativerotation_roll _relativerotation_pitch) (`KismetMathLibrary.BreakRotator` (`SceneComponent.RelativeRotation` (`self.root`))))
  (set `self.TargetPitch` _relativerotation_pitch))

(event `ChangeAngle`
  (params (MoveDirection :type "/Game/Blueprints/Mirror/BP_MirrorEnum Enum"))
  (bind (_relativerotation_roll _relativerotation_pitch _relativerotation_yaw) (`KismetMathLibrary.BreakRotator` (`SceneComponent.RelativeRotation` (`self.root`))))
  (bind (_relativerotation_roll_2 _relativerotation_pitch_2 _relativerotation_yaw_2) (`KismetMathLibrary.BreakRotator` (`SceneComponent.RelativeRotation` (`self.root`))))
  (bind (_relativerotation_roll_3 _relativerotation_pitch_3) (`KismetMathLibrary.BreakRotator` (`SceneComponent.RelativeRotation` (`self.root`))))
  (bind _returnvalue (`KismetMathLibrary.FInterpTo_Constant` _relativerotation_pitch (`self.TargetPitch`) (`GameplayStatics.GetWorldDeltaSeconds`) (`self.AngleChangeSpeed`)))
  ;[1 1 1] Change Angle Up Or Down
  (if (`|EnumEquality` MoveDirection "NewEnumerator0")
    (set `self.AngleChangeAmount` 45.0)
    (else
      (set `self.AngleChangeAmount` -45.0)))
  (bind _output_get (set `self.TargetPitch` (`KismetMathLibrary.FClamp` (+ (`self.AngleChangeAmount`) (`self.TargetPitch`)) -90.0 90.0)))
  (`KismetSystemLibrary.PrintString` (`KismetStringLibrary.Conv_DoubleToString` _output_get))
  (if (not (`self.bChangingAngle`))
    (`|ExecutionSequence`
      (:`then_0`
        (goto _label :!via `Open`))
      (:`then_1`
        (`/Engine/EditorBlueprintResources/StandardMacros.Gate` true :!label _label
          (:`Exit`
            (`SceneComponent.K2_SetRelativeRotation` (`self.root`) (`KismetMathLibrary.MakeRotator` _relativerotation_roll _returnvalue _relativerotation_yaw) false false)
            (`KismetSystemLibrary.Delay` (`GameplayStatics.GetWorldDeltaSeconds`))
            (if (or (>= _relativerotation_pitch_3 90.0) (<= _relativerotation_pitch_3 -90.0))
              (set `self.bChangingAngle` false)
              (`KismetSystemLibrary.PrintString` "Reached")
              (goto _label :!via `Close`)
              (elif (`KismetMathLibrary.NearlyEqual_FloatFloat` _returnvalue (`self.TargetPitch`) 0.1)
                (set `self.bChangingAngle` false)
                (`SceneComponent.K2_SetRelativeRotation` (`self.root`) (`KismetMathLibrary.MakeRotator` _relativerotation_roll_2 (`self.TargetPitch`) _relativerotation_yaw_2) false false)
                (`KismetSystemLibrary.PrintString` "Reached")
                (goto _label :!via `Close`)
                (else
                  (set `self.bChangingAngle` true)
                  (goto _label))))))))))

(event `self.ReceiveActorBeginOverlap`
  (params (OtherActor :type "Actor Object Reference"))
  ;[1 1 1] Change Angle Up Or Down
  (`SkeletalMeshComponent.PlayAnimation` (`self.Tramp`) "/Game/Blueprints/Mirror/Pointing_Tramp_Bounce_Anim_Armature_ActionBounce.Pointing_Tramp_Bounce_Anim_Armature_ActionBounce" false))

(fn `UserConstructionScript`)