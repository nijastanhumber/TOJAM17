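; BP_Chest is a chest that ends the game when a BaseCharacter overlaps its trigger.
; The RotateLid timeline swings the lid open, then plays a 2D sound and shows the UI_GameDone widget.
; After a short delay it resets CurrentLevel on the game instance and game mode, then loads MainMenu.
; An unconnected branch that would show a quit menu never runs.
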(event `self.Trigger.OnComponentBeginOverlap`
  (params (OverlappedComponent :type "PrimitiveComponent Object Reference") (OtherActor :type "Actor Object Reference") (OtherComp :type "PrimitiveComponent Object Reference") (OtherBodyIndex :type Integer) (bFromSweep :type Boolean) (SweepResult :type "HitResult Structure (by ref)"))
  (cast `/Game/Blueprints/Characters/BaseCharacter` OtherActor)
  (bind (_direction _rotation) (`Timeline|RotateLid`)
    (:`Update`
      (`SceneComponent.K2_SetRelativeRotation` (`self.ChestLid`) (`KismetMathLibrary.MakeRotator` 0.0 _rotation) false false))
    (:`Finished`
      (`GameplayStatics.PlaySound2D` "/Game/Sound/LevelSounds/FAILURE.FAILURE")
      (`/Engine/EditorBlueprintResources/StandardMacros.IsValid` (`self.GameDone`)
        (:`Is Valid`
          _)
        (:`Is Not Valid`
          (bind _returnvalue (`|CreateWidget` "/Game/Blueprints/UI/UI_GameDone.UI_GameDone_C"))
          (set `self.GameDone` _returnvalue)))
      (`UserWidget.AddToViewport` (`self.GameDone`) 0)
      (`KismetSystemLibrary.Delay` 3.0)
      (set `/Game/Blueprints/BP_GameInstance.CurrentLevel` 1 (cast `/Game/Blueprints/BP_GameInstance` (`GameplayStatics.GetGameInstance`) :!pure true))
      (set `/Game/Blueprints/BP_GameMode.CurrentLevel` 1 (cast `/Game/Blueprints/BP_GameMode` (`GameplayStatics.GetGameMode`) :!pure true))
      (`GameplayStatics.OpenLevel` "MainMenu"))))

(fn `UserConstructionScript`)