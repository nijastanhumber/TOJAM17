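; BP_Target is a target actor with a rune whose color animates from BeginPlay.
; It creates a dynamic material instance on the Rune component, then plays the RuneColor timeline to drive only the blue channel of its Color parameter.
; A HoverRock timeline would add a position offset to the actor's location, but nothing triggers it, so that movement never runs.
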(event `self.ReceiveBeginPlay`
  (bind _returnvalue (`PrimitiveComponent.CreateDynamicMaterialInstance` (`self.Rune`) 0 null))
  (bind _output_get (set `self.RuneMaterial` _returnvalue))
  (bind (_direction _blue) (`Timeline|RuneColor`)
    (:`Update`
      (bind _returnvalue_2 (`MaterialInstanceDynamic.K2_GetVectorParameterValue` _output_get "Color"))
      (bind (_r _g _b _a) (break `LinearColor` _returnvalue_2))
      (`MaterialInstanceDynamic.SetVectorParameterValue` _returnvalue "Color" (`KismetMathLibrary.MakeColor` _r _g _blue _a))
      (`MaterialInstanceDynamic.SetVectorParameterValue` _output_get "Color" (`KismetMathLibrary.MakeColor` _r _g _blue _a)))))

(fn `UserConstructionScript`)