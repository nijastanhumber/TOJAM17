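; Player bow character that handles aiming and shooting arrows.
; BeginPlay attaches bow, arrow and quiver meshes to sockets, spawns one hidden projectile and starts ambient music.
; Holding SecondaryAction slows walking, shows the hand arrow, plays a pull sound and enables shooting after a half-second delay.
; Shoot fires the reused projectile from the arrow socket, pitched by the spine rotation target, unless it is already in use.
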(event `self.ReceiveBeginPlay`
  (`SceneComponent.K2_AttachToComponent` (`self.BowMesh`) (`self.Mesh`) "WeaponSocket" "KeepRelative" "KeepRelative" "KeepRelative" true)
  (`SceneComponent.K2_AttachToComponent` (`self.ArrowMesh`) (`self.Mesh`) "ArrowSocket" "KeepRelative" "KeepRelative" "KeepRelative" true)
  (`SceneComponent.K2_AttachToComponent` (`self.QuiverMesh`) (`self.Mesh`) "QuiverSocket" "KeepRelative" "KeepRelative" "KeepRelative" true)
  (bind _returnvalue (`|SpawnActorFromClass` "/Game/Blueprints/Projectile/BP_Projectile.BP_Projectile_C" (`KismetMathLibrary.MakeTransform` (0.0 0.0 0.0) (struct) (1.0 1.0 1.0)) "Undefined" "OverrideRootScale"))
  (bind _output_get (set `self.ProjectileOnHand` _returnvalue))
  (`self.SetActorHiddenInGame` _output_get true)
  (`GameplayStatics.PlaySound2D` "/Game/Sound/LevelSounds/Ambience_-_Mystical_beat_loop.Ambience_-_Mystical_beat_loop"))

(event `InputAction|Shoot`
  (params (Key :type "Key Structure" :default "AnyKey"))
  (bind _projectileonhand (`self.ProjectileOnHand`))
  ;[1 1 1] Shoot if holding aiming for 1 second
  (:`Pressed`
    (set `self.Shooting` true)
    (if (`self.CanShoot`)
      (if (not (`/Game/Blueprints/Projectile/BP_Projectile.bInUse` (`self.ProjectileOnHand`)))
        (`self.K2_SetActorLocationAndRotation` _projectileonhand (`SceneComponent.GetSocketLocation` (`self.ArrowMesh`) "ArrowSocket") (`KismetMathLibrary.MakeRotator` 0.0 (* (`self.SpineRotationTarget`) -1.0) (`self.ProjectileFix`)) false false)
        (`/Game/Blueprints/Projectile/BP_Projectile.Fire` _projectileonhand)
        (set `/Game/Blueprints/Projectile/BP_Projectile.bInUse` true _projectileonhand)
        (set `self.CanShoot` false))))
  (:`Released`
    (set `self.Shooting` false)))

(event `InputAction|SecondaryAction`
  (params (Key :type "Key Structure" :default "AnyKey"))
  (bind _arrowmesh (`self.ArrowMesh`))
  (bind _charactermovement (`self.CharacterMovement`))
  ;[1 1 1] Aim Bow By holding right click/L trigger - and Unhide the arrow on hand
  (:`Pressed`
    (if (not (`/Game/Blueprints/Projectile/BP_Projectile.bInUse` (`self.ProjectileOnHand`)))
      (set `self.aimPressed` true)
      (bind _returnvalue (`GameplayStatics.SpawnSound2D` "/Game/Sound/Bow_String_pull.Bow_String_pull"))
      (set `self.PullSound` _returnvalue)
      (set `CharacterMovementComponent.MaxWalkSpeed` (`self.MaxAimSpeed`) _charactermovement)
      (`SceneComponent.SetHiddenInGame` _arrowmesh false false)
      (`KismetSystemLibrary.Delay` 0.5)
      (set `self.CanShoot` true)))
  (:`Released`
    (set `self.aimPressed` false)
    (set `CharacterMovementComponent.MaxWalkSpeed` (`self.MaxMoveSpeed`) _charactermovement)
    (`SceneComponent.SetHiddenInGame` _arrowmesh true false)
    (set `self.CanShoot` false)
    (set `self.SpineRotationTarget` 0.0)
    (`AudioComponent.Stop` (`self.PullSound`))))

(fn `UserConstructionScript`
  (`parent.UserConstructionScript`))