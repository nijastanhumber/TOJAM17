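; BP_ShieldCharacter is a character Blueprint that carries a shield and a sword.
; Its construction script runs the parent's, then attaches ShieldMesh and SwordMesh to the ShieldSocket and WeaponSocket on Mesh, keeping relative transforms.
; BeginPlay repeats both attachments at runtime.
; Tick is empty, and leftover nodes for spine rotation, facing direction and aiming are unconnected, so they never run.
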(event `self.ReceiveBeginPlay`
  (`SceneComponent.K2_AttachToComponent` (`self.ShieldMesh`) (`self.Mesh`) "ShieldSocket" "KeepRelative" "KeepRelative" "KeepRelative" true)
  (`SceneComponent.K2_AttachToComponent` (`self.SwordMesh`) (`self.Mesh`) "WeaponSocket" "KeepRelative" "KeepRelative" "KeepRelative" true))

(event `self.ReceiveTick`
  (params (DeltaSeconds :type "Float (single-precision)")))

(fn `UserConstructionScript`
  (`parent.UserConstructionScript`)
  (`SceneComponent.K2_AttachToComponent` (`self.ShieldMesh`) (`self.Mesh`) "ShieldSocket" "KeepRelative" "KeepRelative" "KeepRelative" true)
  (`SceneComponent.K2_AttachToComponent` (`self.SwordMesh`) (`self.Mesh`) "WeaponSocket" "KeepRelative" "KeepRelative" "KeepRelative" true))